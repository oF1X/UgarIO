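; Destructible box that loses one HP each time its Box component registers a hit.
; When HP reaches zero, it hides and disables collision instead of being destroyed.
; Tick polls the MyPers player character and, while IsDeath is true, restores the box's visibility, collision and HP so it returns after the player dies.
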(event `self.box.OnComponentHit`
  (params (HitComponent :type "PrimitiveComponent Object Reference") (OtherActor :type "Actor Object Reference") (OtherComp :type "PrimitiveComponent Object Reference") (NormalImpulse :type "Vector Structure") (Hit :type "HitResult Structure (by ref)"))
  (bind _box (`self.box`))
  ;[1 1 1] HP object
  (bind _result (`/Engine/EditorBlueprintResources/StandardMacros.DecrementInt` (`self.Hp`))
    (:`  `
      (if (== _result 0)
        (`SceneComponent.SetVisibility` _box false false)
        (`PrimitiveComponent.SetCollisionEnabled` _box "NoCollision")))))

(event `self.ReceiveTick`
  (params (DeltaSeconds :type "Float (single-precision)"))
  (bind _box (`self.box`))
  ;[1 1 1] Востановление объекта после смерти персонажа
  (bind _asmy_pers (cast `/Game/1aaa/Player/MyPers` (`GameplayStatics.GetPlayerCharacter` 0)))
  (if (`/Game/1aaa/Player/MyPers.IsDeath` _asmy_pers)
    (`SceneComponent.SetVisibility` _box true false)
    (`PrimitiveComponent.SetCollisionEnabled` _box "QueryAndPhysics")
    (set `self.Hp` 3)))

(fn `UserConstructionScript`)