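; A breakable secret box that loses Hp on each hit and spawns an HpObj pickup when Hp reaches zero.
; On breaking it hides and disables collision rather than being destroyed.
; Tick polls the player's MyPers and restores visibility, collision and Hp whenever InBox or IsDeath is true.
; After a break, a later non-breaking hit destroys the previously spawned HpObj through a DoOnce that each break resets.
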(event `self.secret_box.OnComponentHit`
  (params (HitComponent :type "PrimitiveComponent Object Reference") (OtherActor :type "Actor Object Reference") (OtherComp :type "PrimitiveComponent Object Reference") (NormalImpulse :type "Vector Structure") (Hit :type "HitResult Structure (by ref)"))
  (bind _returnvalue (`self.GetTransform`))
  (bind _secret_box (`self.secret_box`))
  ;[1 1 1] Destroy and Create HPobj
  (bind _result (`/Engine/EditorBlueprintResources/StandardMacros.DecrementInt` (`self.Hp`))
    (:`  `
      (if (== _result 0)
        (bind _returnvalue_2 (`|SpawnActorFromClass` "/Game/1aaa/Objects/health/HpObj.HpObj_C" (`KismetMathLibrary.MakeTransform` (`KismetMathLibrary.MakeVector` (.x (.location _returnvalue)) (+ (.y (.location _returnvalue)) -5.0) (.z (.location _returnvalue))) (.rotation _returnvalue) (.scale _returnvalue)) "Undefined" "OverrideRootScale" null null))
        (`SceneComponent.SetVisibility` _secret_box false false)
        (`PrimitiveComponent.SetCollisionEnabled` _secret_box "NoCollision")
        (set `self.once` true)
        (goto _label :!via `Reset`)
        (elif (`self.once`)
          (`/Engine/EditorBlueprintResources/StandardMacros.DoOnce` false :!label _label
            (:`Completed`
              (`self.K2_DestroyActor` _returnvalue_2))))))))

(event `self.ReceiveTick`
  (params (DeltaSeconds :type "Float (single-precision)"))
  (bind _secret_box (`self.secret_box`))
  ;[1 1 1] Comment
  (bind _asmy_pers (cast `/Game/1aaa/Player/MyPers` (`GameplayStatics.GetPlayerCharacter` 0)))
  (if (or (`/Game/1aaa/Player/MyPers.InBox` _asmy_pers) (`/Game/1aaa/Player/MyPers.IsDeath` _asmy_pers))
    (`SceneComponent.SetVisibility` _secret_box true false)
    (`PrimitiveComponent.SetCollisionEnabled` _secret_box "QueryAndPhysics")
    (set `self.Hp` 3)))

(fn `UserConstructionScript`)