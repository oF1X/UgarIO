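; DoorBp is a decor door that visually switches between open and closed based on the player character's InBox flag, which an author comment links to having a key.
; Every Tick it casts player 0 to MyPers and toggles visibility on the open and closed top and middle pieces.
; The open look appears after a short Delay, while the closed look applies immediately.
; Only visibility changes, with no animation or collision logic.
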(event `self.ReceiveTick`
  (params (DeltaSeconds :type "Float (single-precision)"))
  (bind _closedtop (`self.closedTop`))
  (bind _closedmid (`self.closedMid`))
  (bind _opentop (`self.openTop`))
  (bind _openmid (`self.openMid`))
  ;[1 1 1] Visible if have key
  (bind _asmy_pers (cast `/Game/1aaa/Player/MyPers` (`GameplayStatics.GetPlayerCharacter` 0)))
  (if (`/Game/1aaa/Player/MyPers.InBox` _asmy_pers)
    (`KismetSystemLibrary.Delay` 0.3)
    (`SceneComponent.SetVisibility` _opentop true false)
    (`SceneComponent.SetVisibility` _openmid true false)
    (`SceneComponent.SetVisibility` _closedmid false false)
    (`SceneComponent.SetVisibility` _closedtop false false)
    (else
      (`SceneComponent.SetVisibility` _closedmid true false)
      (`SceneComponent.SetVisibility` _closedtop true false)
      (`SceneComponent.SetVisibility` _opentop false false)
      (`SceneComponent.SetVisibility` _openmid false false))))

(fn `UserConstructionScript`)